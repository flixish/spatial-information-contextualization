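; Player controller for the Viewer, holding cursor selection logic for meshes and plans, though every node in its Select input graph is disabled.
; The disabled graph traces under the cursor, passes mesh or plan hits to GM_Viewer, clears selection on a miss, and debug-prints other hits.
; TraceForTransparency renders the hit runtime mesh's material to a render target and prints the alpha at the collision UV.
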(fn `TraceForTransparency`
  (bind _hitresult (`self.GetHitResultUnderCursorByChannel` "TraceTypeQuery1"))
  (bind (_x _y) (`KismetMathLibrary.BreakVector2D` (`GameplayStatics.FindCollisionUV` _hitresult)))
  (bind _asruntime_mesh_component_static (cast `RuntimeMeshComponentStatic` (`.HitComponent` (`GameplayStatics.BreakHitResult` _hitresult))))
  (bind _returnvalue (`KismetRenderingLibrary.CreateRenderTarget2D` 1024 1024 "RTF_RGBA8"))
  (`KismetRenderingLibrary.DrawMaterialToRenderTarget` _returnvalue (`PrimitiveComponent.GetMaterial` _asruntime_mesh_component_static 0))
  (bind _returnvalue_2 (`KismetRenderingLibrary.ReadRenderTargetRawUV` _returnvalue _x _y))
  (`KismetSystemLibrary.PrintString` (`KismetStringLibrary.Conv_DoubleToString` (`.A` (`KismetMathLibrary.BreakColor` _returnvalue_2))))
  (return))

(fn `UserConstructionScript`)