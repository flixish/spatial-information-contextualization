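; BP_Plan is a textured plan actor in the viewer that can be selected and repositioned with the mouse.
; SetUpPlan scales and places it with a dynamic material, and UpdateTransform records its location and rotation offsets from that initial transform.
; GM_Viewer selection events toggle its custom depth highlight.
; With Move enabled, clicking attaches it to a spawned BP_Origin that follows the cursor hit on Tick, and clicking again detaches it and clears Move.
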(event `self.ReceiveBeginPlay`
  (bind _asgm_viewer (cast `/Game/Viewer/01_Core/GM_Viewer` (`GameplayStatics.GetGameMode`)))
  (`/Game/Viewer/01_Core/GM_Viewer.RefreshPlanOutliner` _asgm_viewer)
  (add `/Game/Viewer/01_Core/GM_Viewer.SelectPlan` _asgm_viewer (delegate `Select`))
  (add `/Game/Viewer/01_Core/GM_Viewer.SelectViewerMesh` _asgm_viewer (delegate `Deselect`)))

(event `Select`
  (params (Plan :type "/Game/Viewer/01_Core/04_Plan/BP_Plan Object Reference"))
  (`PrimitiveComponent.SetRenderCustomDepth` (`self.Plan`) (== Plan self)))

(event `Deselect`
  (params (ViewerMesh :type "/Game/Viewer/01_Core/Meshes/ViewerMeshActor Object Reference"))
  (`PrimitiveComponent.SetRenderCustomDepth` (`self.Plan`) false))

(event `self.ReceiveTick`
  (params (DeltaSeconds :type "Float (single-precision)"))
  (`/Engine/EditorBlueprintResources/StandardMacros.Gate` true :!label _label
    (:`Exit`
      (`self.K2_SetActorLocation` (`self.Origin`) (`.Location` (`GameplayStatics.BreakHitResult` (`PlayerController.GetHitResultUnderCursorForObjects` (`GameplayStatics.GetPlayerController` 0) (`|MakeArray` "ObjectTypeQuery1" "ObjectTypeQuery2" :!type "EObjectTypeQuery Enum") true))) false false))))

(event `self.Plan.OnClicked`
  (params (TouchedComponent :type "PrimitiveComponent Object Reference") (ButtonPressed :type "Key Structure"))
  (if (`self.bMove`)
    (bind _returnvalue (`|SpawnActorFromClass` "/Game/Viewer/01_Core/04_Plan/BP_Origin.BP_Origin_C" (`KismetMathLibrary.MakeTransform` (`.Location` (`GameplayStatics.BreakHitResult` (`PlayerController.GetHitResultUnderCursorByChannel` (`GameplayStatics.GetPlayerController` 0) "TraceTypeQuery1" true)))) "Undefined" "OverrideRootScale" null null))
    (set `self.Origin` _returnvalue)
    (`|MultiGate` false true
      (:`Out 0`
        (`self.K2_AttachToActor` (`self.Origin`) "None" "KeepWorld" "KeepWorld" "KeepWorld")
        (goto _label :!via `Open`))
      (:`Out 1`
        (set `self.bMove` false)
        (`self.K2_DetachFromActor` "KeepWorld" "KeepWorld" "KeepWorld")
        (`self.K2_DestroyActor` (`self.Origin`))
        (goto _label :!via `Close`)))))

(fn `SetUpPlan`
  (params (SizeX :type Integer) (SizeY :type Integer) (Texture :type "Texture2D Object Reference") (Transform :type "Transform Structure (by ref)"))
  (set `self.Texture` Texture)
  (`SceneComponent.SetRelativeScale3D` (`self.Plan`) (`KismetMathLibrary.MakeVector` (/ (`KismetMathLibrary.Conv_IntToDouble` SizeX) 10.0) (/ (`KismetMathLibrary.Conv_IntToDouble` SizeY) 10.0) 1.0))
  (`self.K2_SetActorTransform` Transform)
  (set `self.InitialTransform` Transform)
  (bind _returnvalue (`KismetMaterialLibrary.CreateDynamicMaterialInstance` "/Game/Viewer/01_Core/04_Plan/M_PlanMaterial.M_PlanMaterial"))
  (`MaterialInstanceDynamic.SetTextureParameterValue` _returnvalue "Texture" (`local.Texture`))
  (`PrimitiveComponent.SetMaterial` (`self.Plan`) 0 _returnvalue))

(fn `UpdateTransform`
  (bind _output_get (set `self.UpdatedTransform` (`self.GetTransform`)))
  (set `self.LocationDifference` (- (.location _output_get) (.location (`self.InitialTransform`))))
  (set `self.RotationDifference` (`KismetMathLibrary.NormalizedDeltaRotator` (.rotation _output_get) (.rotation (`self.InitialTransform`)))))

(fn `UserConstructionScript`)