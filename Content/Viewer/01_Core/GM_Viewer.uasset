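; Viewer game mode that seeds the building-part hierarchy and tracks which part is selected.
; BeginPlay builds a hard-coded church partonomy of nested BPO_BuildingPartCollection objects under the first BPA_BuildingHierarchy's root, tagged with GUIDs, existence years and some Getty subject terms.
; Hierarchy selection stores the chosen part and enables the main UI's edit button.
; Save/load logic for 3D boxes and collections, with recursive helpers, is unwired and incomplete.
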(event `SaveGameLoad`)

(event `self.ReceiveBeginPlay`
  (add `self.SelectedHierarchyEntry` (delegate `SetCurrentHierarchySelection`))
  ;[1 1 1] Construct empty BuildingPartCollection
  (bind _outactors (`GameplayStatics.GetAllActorsOfClass` "/Game/Viewer/01_Core/01_Partonomie/BPA_BuildingHierarchy.BPA_BuildingHierarchy_C"))
  (bind _output_get (set `self.BuildingHierarchies` _outactors))
  (bind _rootbuildingpartcollection (`/Game/Viewer/01_Core/01_Partonomie/BPA_BuildingHierarchy.GetRootBuildingPartCollection` (`|GetArrayItem` _output_get)))
  (set `self.BauwerksCollection` _rootbuildingpartcollection)
  (bind _returnvalue (`|GenericCreateObject` "/Game/Viewer/01_Core/01_Partonomie/BPO_BuildingPartCollection.BPO_BuildingPartCollection_C" "/Game/Viewer/01_Core/01_Partonomie/BPA_BuildingHierarchy_01.BPA_BuildingHierarchy_01" (make `/Game/Viewer/01_Core/Structs/S_BuildingPart` (`KismetGuidLibrary.NewGuid`) "Bauwerk" "" "" null false _ (`self.ExistenceStart`) (`self.ExistenceEnd`))))
  (`/Game/Viewer/01_Core/01_Partonomie/BPO_BuildingPartCollection.AddSubBuildingPartCollection` _rootbuildingpartcollection _returnvalue)
  ;[1 1 1] ManualLoadedPartonomie
  (bind _returnvalue_2 (`|GenericCreateObject` "/Game/Viewer/01_Core/01_Partonomie/BPO_BuildingPartCollection.BPO_BuildingPartCollection_C" "/Game/Viewer/01_Core/01_Partonomie/BPA_BuildingHierarchy_01.BPA_BuildingHierarchy_01" (make `/Game/Viewer/01_Core/Structs/S_BuildingPart` (`KismetGuidLibrary.NewGuid`) "Foyer" "300004263" "entrance halls" null false _ 1966 0 _returnvalue)))
  (`/Game/Viewer/01_Core/01_Partonomie/BPO_BuildingPartCollection.AddSubBuildingPartCollection` _returnvalue _returnvalue_2)
  (bind _returnvalue_3 (`|GenericCreateObject` "/Game/Viewer/01_Core/01_Partonomie/BPO_BuildingPartCollection.BPO_BuildingPartCollection_C" "/Game/Viewer/01_Core/01_Partonomie/BPA_BuildingHierarchy_01.BPA_BuildingHierarchy_01" (make `/Game/Viewer/01_Core/Structs/S_BuildingPart` (`KismetGuidLibrary.NewGuid`) "Großer Saal" "300004420" "halls (interior spaces)" null false _ 1966)))
  (bind _returnvalue_4 (`|GenericCreateObject` "/Game/Viewer/01_Core/01_Partonomie/BPO_BuildingPartCollection.BPO_BuildingPartCollection_C" "/Game/Viewer/01_Core/01_Partonomie/BPA_BuildingHierarchy_01.BPA_BuildingHierarchy_01" (make `/Game/Viewer/01_Core/Structs/S_BuildingPart` (`KismetGuidLibrary.NewGuid`) "Musikbereich" "300100084" "forestages" null false _ 1966)))
  (`/Game/Viewer/01_Core/01_Partonomie/BPO_BuildingPartCollection.AddSubBuildingPartCollection` _returnvalue_3 _returnvalue_4)
  (bind _returnvalue_5 (`|GenericCreateObject` "/Game/Viewer/01_Core/01_Partonomie/BPO_BuildingPartCollection.BPO_BuildingPartCollection_C" "/Game/Viewer/01_Core/01_Partonomie/BPA_BuildingHierarchy_01.BPA_BuildingHierarchy_01" (make `/Game/Viewer/01_Core/Structs/S_BuildingPart` (`KismetGuidLibrary.NewGuid`) "Wandfläche 1" "300081138" "adobe bricks" null false _ 1966)))
  (`/Game/Viewer/01_Core/01_Partonomie/BPO_BuildingPartCollection.AddSubBuildingPartCollection` _returnvalue_4 _returnvalue_5)
  (bind _returnvalue_6 (`|GenericCreateObject` "/Game/Viewer/01_Core/01_Partonomie/BPO_BuildingPartCollection.BPO_BuildingPartCollection_C" "/Game/Viewer/01_Core/01_Partonomie/BPA_BuildingHierarchy_01.BPA_BuildingHierarchy_01" (make `/Game/Viewer/01_Core/Structs/S_BuildingPart` (`KismetGuidLibrary.NewGuid`) "Wandfläche 2" "300081138" "adobe bricks" null false _ 1966)))
  (`/Game/Viewer/01_Core/01_Partonomie/BPO_BuildingPartCollection.AddSubBuildingPartCollection` _returnvalue_4 _returnvalue_6)
  (bind _returnvalue_7 (`|GenericCreateObject` "/Game/Viewer/01_Core/01_Partonomie/BPO_BuildingPartCollection.BPO_BuildingPartCollection_C" "/Game/Viewer/01_Core/01_Partonomie/BPA_BuildingHierarchy_01.BPA_BuildingHierarchy_01" (make `/Game/Viewer/01_Core/Structs/S_BuildingPart` (`KismetGuidLibrary.NewGuid`) "Wandfläche 3" "300081138" "adobe bricks" null false _ 1966)))
  (`/Game/Viewer/01_Core/01_Partonomie/BPO_BuildingPartCollection.AddSubBuildingPartCollection` _returnvalue_4 _returnvalue_7)
  (bind _returnvalue_8 (`|GenericCreateObject` "/Game/Viewer/01_Core/01_Partonomie/BPO_BuildingPartCollection.BPO_BuildingPartCollection_C" "/Game/Viewer/01_Core/01_Partonomie/BPA_BuildingHierarchy_01.BPA_BuildingHierarchy_01" (make `/Game/Viewer/01_Core/Structs/S_BuildingPart` (`KismetGuidLibrary.NewGuid`) "Fenster" "300002944" "windows" null false _ 1966)))
  (`/Game/Viewer/01_Core/01_Partonomie/BPO_BuildingPartCollection.AddSubBuildingPartCollection` _returnvalue_6 _returnvalue_8)
  (bind _returnvalue_9 (`|GenericCreateObject` "/Game/Viewer/01_Core/01_Partonomie/BPO_BuildingPartCollection.BPO_BuildingPartCollection_C" "/Game/Viewer/01_Core/01_Partonomie/BPA_BuildingHierarchy_01.BPA_BuildingHierarchy_01" (make `/Game/Viewer/01_Core/Structs/S_BuildingPart` (`KismetGuidLibrary.NewGuid`) "Fenster 1" "300002944" "windows" null false _ 1966)))
  (`/Game/Viewer/01_Core/01_Partonomie/BPO_BuildingPartCollection.AddSubBuildingPartCollection` _returnvalue_7 _returnvalue_9)
  (bind _returnvalue_10 (`|GenericCreateObject` "/Game/Viewer/01_Core/01_Partonomie/BPO_BuildingPartCollection.BPO_BuildingPartCollection_C" "/Game/Viewer/01_Core/01_Partonomie/BPA_BuildingHierarchy_01.BPA_BuildingHierarchy_01" (make `/Game/Viewer/01_Core/Structs/S_BuildingPart` (`KismetGuidLibrary.NewGuid`) "Fenster 2" "300002944" "windows" null false _ 1966)))
  (`/Game/Viewer/01_Core/01_Partonomie/BPO_BuildingPartCollection.AddSubBuildingPartCollection` _returnvalue_7 _returnvalue_10)
  (bind _returnvalue_11 (`|GenericCreateObject` "/Game/Viewer/01_Core/01_Partonomie/BPO_BuildingPartCollection.BPO_BuildingPartCollection_C" "/Game/Viewer/01_Core/01_Partonomie/BPA_BuildingHierarchy_01.BPA_BuildingHierarchy_01" (make `/Game/Viewer/01_Core/Structs/S_BuildingPart` (`KismetGuidLibrary.NewGuid`) "Fenster 3" "300002944" "windows" null false _ 1966)))
  (`/Game/Viewer/01_Core/01_Partonomie/BPO_BuildingPartCollection.AddSubBuildingPartCollection` _returnvalue_7 _returnvalue_11)
  (bind _returnvalue_12 (`|GenericCreateObject` "/Game/Viewer/01_Core/01_Partonomie/BPO_BuildingPartCollection.BPO_BuildingPartCollection_C" "/Game/Viewer/01_Core/01_Partonomie/BPA_BuildingHierarchy_01.BPA_BuildingHierarchy_01" (make `/Game/Viewer/01_Core/Structs/S_BuildingPart` (`KismetGuidLibrary.NewGuid`) "Altarbereich" "" "" null false _ 1966)))
  (`/Game/Viewer/01_Core/01_Partonomie/BPO_BuildingPartCollection.AddSubBuildingPartCollection` _returnvalue_3 _returnvalue_12)
  (bind _returnvalue_13 (`|GenericCreateObject` "/Game/Viewer/01_Core/01_Partonomie/BPO_BuildingPartCollection.BPO_BuildingPartCollection_C" "/Game/Viewer/01_Core/01_Partonomie/BPA_BuildingHierarchy_01.BPA_BuildingHierarchy_01" (make `/Game/Viewer/01_Core/Structs/S_BuildingPart` (`KismetGuidLibrary.NewGuid`) "Altar" "300003725" "altars (religious fixtures)" null false _ 1966)))
  (`/Game/Viewer/01_Core/01_Partonomie/BPO_BuildingPartCollection.AddSubBuildingPartCollection` _returnvalue_12 _returnvalue_13)
  (bind _returnvalue_14 (`|GenericCreateObject` "/Game/Viewer/01_Core/01_Partonomie/BPO_BuildingPartCollection.BPO_BuildingPartCollection_C" "/Game/Viewer/01_Core/01_Partonomie/BPA_BuildingHierarchy_01.BPA_BuildingHierarchy_01" (make `/Game/Viewer/01_Core/Structs/S_BuildingPart` (`KismetGuidLibrary.NewGuid`) "Rückwand" "" "" null false _ 1966)))
  (`/Game/Viewer/01_Core/01_Partonomie/BPO_BuildingPartCollection.AddSubBuildingPartCollection` _returnvalue_12 _returnvalue_14)
  (bind _returnvalue_15 (`|GenericCreateObject` "/Game/Viewer/01_Core/01_Partonomie/BPO_BuildingPartCollection.BPO_BuildingPartCollection_C" "/Game/Viewer/01_Core/01_Partonomie/BPA_BuildingHierarchy_01.BPA_BuildingHierarchy_01" (make `/Game/Viewer/01_Core/Structs/S_BuildingPart` (`KismetGuidLibrary.NewGuid`) "Triptychon" "" "" null false _ 1966)))
  (`/Game/Viewer/01_Core/01_Partonomie/BPO_BuildingPartCollection.AddSubBuildingPartCollection` _returnvalue_14 _returnvalue_15)
  (bind _returnvalue_16 (`|GenericCreateObject` "/Game/Viewer/01_Core/01_Partonomie/BPO_BuildingPartCollection.BPO_BuildingPartCollection_C" "/Game/Viewer/01_Core/01_Partonomie/BPA_BuildingHierarchy_01.BPA_BuildingHierarchy_01" (make `/Game/Viewer/01_Core/Structs/S_BuildingPart` (`KismetGuidLibrary.NewGuid`) "Lichtwand" "" "" null false _ 1966)))
  (`/Game/Viewer/01_Core/01_Partonomie/BPO_BuildingPartCollection.AddSubBuildingPartCollection` _returnvalue_3 _returnvalue_16)
  (`/Game/Viewer/01_Core/01_Partonomie/BPO_BuildingPartCollection.AddSubBuildingPartCollection` _returnvalue _returnvalue_3)
  (bind _returnvalue_17 (`|GenericCreateObject` "/Game/Viewer/01_Core/01_Partonomie/BPO_BuildingPartCollection.BPO_BuildingPartCollection_C" "/Game/Viewer/01_Core/01_Partonomie/BPA_BuildingHierarchy_01.BPA_BuildingHierarchy_01" (make `/Game/Viewer/01_Core/Structs/S_BuildingPart` (`KismetGuidLibrary.NewGuid`) "Sakristei" "300004631" "sacristies (religious spaces)" null false _ 1966)))
  (`/Game/Viewer/01_Core/01_Partonomie/BPO_BuildingPartCollection.AddSubBuildingPartCollection` _returnvalue _returnvalue_17)
  (bind _returnvalue_18 (`|GenericCreateObject` "/Game/Viewer/01_Core/01_Partonomie/BPO_BuildingPartCollection.BPO_BuildingPartCollection_C" "/Game/Viewer/01_Core/01_Partonomie/BPA_BuildingHierarchy_01.BPA_BuildingHierarchy_01" (make `/Game/Viewer/01_Core/Structs/S_BuildingPart` (`KismetGuidLibrary.NewGuid`) "Innenhof" "300004095" "courtyards" null false _ 1966)))
  (`/Game/Viewer/01_Core/01_Partonomie/BPO_BuildingPartCollection.AddSubBuildingPartCollection` _returnvalue _returnvalue_18)
  (bind _returnvalue_19 (`|GenericCreateObject` "/Game/Viewer/01_Core/01_Partonomie/BPO_BuildingPartCollection.BPO_BuildingPartCollection_C" "/Game/Viewer/01_Core/01_Partonomie/BPA_BuildingHierarchy_01.BPA_BuildingHierarchy_01" (make `/Game/Viewer/01_Core/Structs/S_BuildingPart` (`KismetGuidLibrary.NewGuid`) "Kapelle" "300004590" "chapels (rooms or structures)" null false _ 1966)))
  (`/Game/Viewer/01_Core/01_Partonomie/BPO_BuildingPartCollection.AddSubBuildingPartCollection` _returnvalue _returnvalue_19)
  (bind _returnvalue_20 (`|GenericCreateObject` "/Game/Viewer/01_Core/01_Partonomie/BPO_BuildingPartCollection.BPO_BuildingPartCollection_C" "/Game/Viewer/01_Core/01_Partonomie/BPA_BuildingHierarchy_01.BPA_BuildingHierarchy_01" (make `/Game/Viewer/01_Core/Structs/S_BuildingPart` (`KismetGuidLibrary.NewGuid`) "Bauernhaus Schulte-Vels" "300005574" "farmhouses (rural houses)" null false _ 1966)))
  (`/Game/Viewer/01_Core/01_Partonomie/BPO_BuildingPartCollection.AddSubBuildingPartCollection` _returnvalue _returnvalue_20)
  (bind _returnvalue_21 (`|GenericCreateObject` "/Game/Viewer/01_Core/01_Partonomie/BPO_BuildingPartCollection.BPO_BuildingPartCollection_C" "/Game/Viewer/01_Core/01_Partonomie/BPA_BuildingHierarchy_01.BPA_BuildingHierarchy_01" (make `/Game/Viewer/01_Core/Structs/S_BuildingPart` (`KismetGuidLibrary.NewGuid`) "Zwischenraum Lichtwand" "" "" null false _ 2014)))
  (`/Game/Viewer/01_Core/01_Partonomie/BPO_BuildingPartCollection.AddSubBuildingPartCollection` _returnvalue _returnvalue_21))

(event `SetCurrentHierarchySelection` :!signature `self.SelectedHierarchyEntry`
  (params (SelectedHierarchyEntry :type "/Game/Viewer/01_Core/01_Partonomie/BPO_BuildingPart Object Reference"))
  (set `self.SelectedBuildingPart` SelectedHierarchyEntry)
  (bind _foundwidgets (`WidgetBlueprintLibrary.GetAllWidgetsOfClass` "/Game/Viewer/02_UI/WBP_MainUI.WBP_MainUI_C"))
  (`Widget.SetIsEnabled` (`/Game/Viewer/02_UI/WBP_MainUI.BuildingPartEditButton` (`|GetArrayItem` _foundwidgets)) true))

(fn `BuildCollectionsLoop`
  (params (InputCollection :type "Array of /Game/Viewer/01_Core/01_Partonomie/BPO_BuildingPartCollection Object Reference"))
  (returns (OutputSubCollection :type "Array of /Game/Viewer/01_Core/01_Partonomie/BPO_BuildingPartCollection Object Reference"))
  (if (!= (`KismetArrayLibrary.Array_Length` InputCollection) 0)
    (for _array_element InputCollection
      (`|GenericCreateObject` "/Game/Viewer/01_Core/01_Partonomie/BPO_BuildingPartCollection.BPO_BuildingPartCollection_C" self (`/Game/Viewer/01_Core/01_Partonomie/BPO_BuildingPart.BuildingPartVariables` _array_element))
      (`self.LoopThroughCollections` (`/Game/Viewer/01_Core/01_Partonomie/BPO_BuildingPartCollection.SubParts` _array_element)))))

(fn `LoopThroughCollections`
  (params (InputCollection :type "Array of /Game/Viewer/01_Core/01_Partonomie/BPO_BuildingPartCollection Object Reference"))
  (returns (OutputSubCollection :type "Array of /Game/Viewer/01_Core/01_Partonomie/BPO_BuildingPartCollection Object Reference"))
  (if (!= (`KismetArrayLibrary.Array_Length` InputCollection) 0)
    (for _array_element InputCollection
      (`KismetArrayLibrary.Array_Add` (`self.CurrentBuildingPartCollections`) _array_element)
      (`self.LoopThroughCollections` (`/Game/Viewer/01_Core/01_Partonomie/BPO_BuildingPartCollection.SubParts` _array_element)))))

(fn `UserConstructionScript`)