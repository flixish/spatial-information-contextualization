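; BP_CsvExporter writes the viewer's building parts, 3D boxes and linked files to index.csv and links.csv in the game root directory.
; ExportCSV gathers parts through GM_Viewer's hierarchy traversal, boxes from the level and files from each part.
; Helper functions turn these into InternalDocument rows, joined with container, person, organisation and linkset header rows.
; Parts with a box or files get GUID-tagged LinkElements grouped under one Link.
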(event `ExportCSV`
  (bind _seperatortype (`self.SeperatorType`))
  (bind _2_person (`self.2_Person`))
  (bind _1_containerdescription (`self.1_ContainerDescription`))
  (bind _3_organisation (`self.3_Organisation`))
  (bind _4_linkset (`self.4_Linkset`))
  (bind _seperatortype_2 (`self.SeperatorType`))
  (bind _masterindexarray (`self.MasterIndexArray`))
  (bind _seperatortype_3 (`self.SeperatorType`))
  (bind _masterlinksarray (`self.MasterLinksArray`))
  (bind _creator (`self.Creator`))
  (bind _seperatortype_4 (`self.SeperatorType`))
  (bind _seperatortype_5 (`self.SeperatorType`))
  (bind _publisher (`self.Publisher`))
  (bind _seperatortype_6 (`self.SeperatorType`))
  (bind _internaldocumentids (`self.InternalDocumentIDs`))
  (`|ExecutionSequence`
    (:`then_0`
      ;[1 1 1] Collet Objects for Export
      ;;[1 1 1] Collect BuildingParts
      (bind _asgm_viewer (cast `/Game/Viewer/01_Core/GM_Viewer` (`GameplayStatics.GetGameMode`)))
      (bind _currentbuildingpartcollections (`/Game/Viewer/01_Core/GM_Viewer.CurrentBuildingPartCollections` _asgm_viewer))
      (`KismetArrayLibrary.Array_Clear` _currentbuildingpartcollections)
      (`/Game/Viewer/01_Core/GM_Viewer.LoopThroughCollections` _asgm_viewer (`/Game/Viewer/01_Core/01_Partonomie/BPO_BuildingPartCollection.SubParts` (`/Game/Viewer/01_Core/01_Partonomie/BPA_BuildingHierarchy.GetRootBuildingPartCollection` (`|GetArrayItem` (`/Game/Viewer/01_Core/GM_Viewer.BuildingHierarchies` _asgm_viewer)))))
      (set `self.BuildingPartsCollection` _currentbuildingpartcollections)
      (`self.CreateBuildingPartStringArrays` (`self.BuildingPartsCollection`)))
    (:`then_1`
      ;;[1 1 1] Collect 3dBoxes
      (bind _outactors (`GameplayStatics.GetAllActorsOfClass` "/Game/Viewer/01_Core/02_3dBox/BP_3dBox.BP_3dBox_C"))
      (bind _output_get (set `self.3dBoxes` _outactors))
      (`self.Create3dBoxesArrays` _output_get))
    (:`then_2`
      ;;[1 1 1] Collect LinkedFiles
      (for _array_element (`self.BuildingPartsCollection`)
        (bind (_buildingpartvariables_buildingpartid _buildingpartvariables_name _buildingpartvariables_gettysubjectid _buildingpartvariables_gettysubjectterm _buildingpartvariables_3dbox _buildingpartvariables_has3d _buildingpartvariables_linkedfiles) (break `/Game/Viewer/01_Core/Structs/S_BuildingPart` (`/Game/Viewer/01_Core/01_Partonomie/BPO_BuildingPart.BuildingPartVariables` _array_element)))
        ;;;[1 1 1] GetFileObjects from BuildingPart
        (if (> (`KismetArrayLibrary.Array_Length` _buildingpartvariables_linkedfiles) 0)
          (for _array_element_2 _buildingpartvariables_linkedfiles
            (`KismetArrayLibrary.Array_Add` (`self.LinkedFilesCollection`) _array_element_2))
          (`self.CreateLinkedFilesCollectionArrays` (`self.LinkedFilesCollection`)))))
    (:`then_3`
      ;[1 1 1] ArrayToString, Then add to MasterArray
      (`|ExecutionSequence`
        (:`then_0`
          (`KismetArrayLibrary.Array_Add` _masterindexarray (`KismetStringLibrary.JoinStringArray` (`self.0_Header`) _seperatortype_3)))
        (:`then_2`
          (`/Engine/EditorBlueprintResources/StandardMacros.DoOnce` false
            (:`Completed`
              (`KismetArrayLibrary.Array_Insert` _1_containerdescription (`self.Creator`) 2)
              (`KismetArrayLibrary.Array_Insert` _1_containerdescription (`KismetStringLibrary.JoinStringArray` _internaldocumentids ",  ") 6)
              (`KismetArrayLibrary.Array_Insert` _1_containerdescription (`self.GetDateTimeStringAppend`) 10)
              (`KismetArrayLibrary.Array_Insert` _1_containerdescription (`self.Publisher`) 11))))
        (:`then_3`
          (`KismetArrayLibrary.Array_Add` _masterindexarray (`KismetStringLibrary.JoinStringArray` _1_containerdescription _seperatortype_3))
          (`KismetSystemLibrary.PrintString` (`KismetStringLibrary.Conv_IntToString` (`KismetArrayLibrary.Array_Length` _internaldocumentids))))
        (:`then_4`
          (`/Engine/EditorBlueprintResources/StandardMacros.DoOnce` false
            (:`Completed`
              (`KismetArrayLibrary.Array_Insert` _2_person _creator 1)
              (`KismetArrayLibrary.Array_Insert` _2_person _creator 2)
              (`KismetArrayLibrary.Array_Insert` _2_person (`self.Publisher`) 11))))
        (:`then_5`
          (`KismetArrayLibrary.Array_Add` _masterindexarray (`KismetStringLibrary.JoinStringArray` _2_person _seperatortype_3)))
        (:`then_6`
          (`/Engine/EditorBlueprintResources/StandardMacros.DoOnce` false
            (:`Completed`
              (`KismetArrayLibrary.Array_Insert` _3_organisation _publisher 1)
              (`KismetArrayLibrary.Array_Insert` _3_organisation _publisher 2)
              (`KismetArrayLibrary.Array_Insert` _3_organisation _publisher 11))))
        (:`then_7`
          (`KismetArrayLibrary.Array_Add` _masterindexarray (`KismetStringLibrary.JoinStringArray` _3_organisation _seperatortype_3)))
        (:`then_8`
          (`/Engine/EditorBlueprintResources/StandardMacros.DoOnce` false
            (:`Completed`
              (`KismetArrayLibrary.Array_Insert` _4_linkset (`self.Creator`) 2)
              (`KismetArrayLibrary.Array_Insert` _4_linkset (`self.GetDateTimeStringAppend`) 10)
              (`KismetArrayLibrary.Array_Insert` _4_linkset _publisher 11))))
        (:`then_9`
          (`KismetArrayLibrary.Array_Add` _masterindexarray (`KismetStringLibrary.JoinStringArray` _4_linkset _seperatortype_3)))
        (:`then_10`
          (`KismetArrayLibrary.Array_Append` _masterindexarray (`self.5_InternalDocument`)))
        (:`then_11`
          ;[1 1 1] Write Index CSV
          (`VictoryBPFunctionLibrary.FileIO__SaveStringArrayToFile` (`VictoryBPFunctionLibrary.VictoryPaths__GameRootDirectory`) "index.csv" (`self.MasterIndexArray`) true)
          (for _array_element_3 (`self.MasterIndexArray`)
            (`KismetSystemLibrary.PrintString` _array_element_3)))
        (:`then_12`
          ;[1 1 1] BuildFileHeader
          (`KismetArrayLibrary.Array_Add` (`self.MasterLinksArray`) (`VictoryBPFunctionLibrary.AppendMultiple` "Type" _seperatortype_2 "GUID" _seperatortype_2 "createdBy" _seperatortype_2 "creationDate" _seperatortype_2 "versionDescription" _seperatortype_2 "hasDocument" _seperatortype_2 "hasLinkElement"))
          (for _array_element_4 (`self.BuildingPartsCollection`)
            (bind (_buildingpartvariables_buildingpartid_2 _buildingpartvariables_name_2 _buildingpartvariables_gettysubjectid_2 _buildingpartvariables_gettysubjectterm_2 _buildingpartvariables_3dbox_2 _buildingpartvariables_has3d_2 _buildingpartvariables_linkedfiles_2) (break `/Game/Viewer/01_Core/Structs/S_BuildingPart` (`/Game/Viewer/01_Core/01_Partonomie/BPO_BuildingPart.BuildingPartVariables` _array_element_4)))
            (bind _returnvalue (> (`KismetArrayLibrary.Array_Length` _buildingpartvariables_linkedfiles_2) 0))
            (if (or (`KismetSystemLibrary.IsValid` _buildingpartvariables_3dbox_2) _returnvalue)
              (`|ExecutionSequence`
                (:`then_0`
                  (bind _output_get_2 (set `self.GuidLocal` (`KismetGuidLibrary.NewGuid`)))
                  (bind _returnvalue_2 (`KismetGuidLibrary.Conv_GuidToString` _output_get_2))
                  (`KismetArrayLibrary.Array_Add` (`self.MasterLinksArray`) (`VictoryBPFunctionLibrary.AppendMultiple` "LinkElement" _seperatortype_4 _returnvalue_2 _seperatortype_4 (`self.Creator`) _seperatortype_4 (`self.GetDateTimeStringAppend`) _seperatortype_4 "Version 1.0" _seperatortype_4 (`KismetGuidLibrary.Conv_GuidToString` _buildingpartvariables_buildingpartid_2)))
                  (`KismetArrayLibrary.Array_Add` (`self.LinkElementIDs`) _returnvalue_2))
                (:`then_1`
                  ;[1 1 1] CreateBoxLinkElement
                  (`/Engine/EditorBlueprintResources/StandardMacros.IsValid` _buildingpartvariables_3dbox_2
                    (:`Is Valid`
                      (bind _output_get_3 (set `self.GuidLocal` (`KismetGuidLibrary.NewGuid`)))
                      (bind _returnvalue_3 (`KismetGuidLibrary.Conv_GuidToString` _output_get_3))
                      (bind _boxcontainervariables_containerid (break `/Game/Viewer/01_Core/Structs/S_3dBox` (`/Game/Viewer/01_Core/02_3dBox/BP_3dBox.BoxContainerVariables` _buildingpartvariables_3dbox_2)))
                      (`KismetArrayLibrary.Array_Add` (`self.MasterLinksArray`) (`VictoryBPFunctionLibrary.AppendMultiple` "LinkElement" _seperatortype_6 _returnvalue_3 _seperatortype_6 (`self.Creator`) _seperatortype_6 (`self.GetDateTimeStringAppend`) _seperatortype_6 "Version 1.0" _seperatortype_6 (`KismetGuidLibrary.Conv_GuidToString` _boxcontainervariables_containerid)))
                      (`KismetArrayLibrary.Array_Add` (`self.LinkElementIDs`) _returnvalue_3))))
                (:`then_2`
                  ;[1 1 1] CreateLinkedFileLinkElement
                  (if _returnvalue
                    (for _array_element_5 _buildingpartvariables_linkedfiles_2
                      (bind _output_get_4 (set `self.GuidLocal` (`KismetGuidLibrary.NewGuid`)))
                      (bind _returnvalue_4 (`KismetGuidLibrary.Conv_GuidToString` _output_get_4))
                      (bind _linkedfilevars_fileguid (break `/Game/Viewer/01_Core/Structs/S_File` (`/Game/Viewer/01_Core/00_LinkedDocuments/BP_LinkedFile.LinkedFileVars` _array_element_5)))
                      (`KismetArrayLibrary.Array_Add` (`self.MasterLinksArray`) (`VictoryBPFunctionLibrary.AppendMultiple` "LinkElement" _seperatortype_5 _returnvalue_4 _seperatortype_5 (`self.Creator`) _seperatortype_5 (`self.GetDateTimeStringAppend`) _seperatortype_5 "Version 1.0" _seperatortype_5 (`KismetGuidLibrary.Conv_GuidToString` _linkedfilevars_fileguid)))
                      (`KismetArrayLibrary.Array_Add` (`self.LinkElementIDs`) _returnvalue_4))))
                (:`then_3`
                  ;[1 1 1] CreateLinkSet
                  (bind _output_get_5 (set `self.GuidLocal` (`KismetGuidLibrary.NewGuid`)))
                  (`KismetArrayLibrary.Array_Add` (`self.MasterLinksArray`) (`VictoryBPFunctionLibrary.AppendMultiple` "Link" _seperatortype (`KismetGuidLibrary.Conv_GuidToString` _output_get_5) _seperatortype (`self.Creator`) _seperatortype (`self.GetDateTimeStringAppend`) _seperatortype "Version 1.0" _seperatortype _seperatortype (`KismetStringLibrary.JoinStringArray` (`self.LinkElementIDs`) ", ")))
                  (`KismetArrayLibrary.Array_Clear` (`self.LinkElementIDs`)))))))
        (:`then_13`
          ;[1 1 1] Write Link CSV
          (`VictoryBPFunctionLibrary.FileIO__SaveStringArrayToFile` (`VictoryBPFunctionLibrary.VictoryPaths__GameRootDirectory`) "links.csv" _masterlinksarray true)
          (for _array_element_6 _masterlinksarray
            (`KismetSystemLibrary.PrintString` _array_element_6)))
        (:`then_14`
          ;[1 1 1] ClearArrays
          (`KismetArrayLibrary.Array_Clear` (`self.MasterIndexArray`))
          (`KismetArrayLibrary.Array_Clear` (`self.5_InternalDocument`))
          (`KismetArrayLibrary.Array_Clear` (`self.InternalDocumentIDs`))
          (`KismetArrayLibrary.Array_Clear` (`self.MasterLinksArray`))
          (`KismetArrayLibrary.Array_Clear` (`self.LinkElementIDs`))
          (`KismetArrayLibrary.Array_Clear` (`self.BuildingPartsCollection`))
          (`KismetArrayLibrary.Array_Clear` (`self.LinkedFilesCollection`))
          (`KismetArrayLibrary.Array_Clear` (`self.3dBoxes`))
          (`KismetSystemLibrary.PrintString` "FINISHED" true true (struct :`G` 0.66 :`B` 1.0 :`A` 1.0) 10.0))))))

(fn `Create3dBoxesArrays`
  (params (Input3dBoxes :type "Array of /Game/Viewer/01_Core/02_3dBox/BP_3dBox Object Reference"))
  (bind _seperatortype (`self.SeperatorType`))
  ;[1 1 1] Create LinkedFiles StringArray
  (for _array_element Input3dBoxes
    (bind (_boxcontainervariables_containerid _boxcontainervariables_buildingpart) (break `/Game/Viewer/01_Core/Structs/S_3dBox` (`/Game/Viewer/01_Core/02_3dBox/BP_3dBox.BoxContainerVariables` _array_element)))
    (bind _returnvalue (`KismetGuidLibrary.Conv_GuidToString` _boxcontainervariables_containerid))
    (`KismetArrayLibrary.Array_Add` (`self.InternalDocumentIDs`) _returnvalue)
    (bind _returnvalue_2 (`KismetStringLibrary.Conv_DoubleToString` (.x (.scale (`SceneComponent.K2_GetComponentToWorld` (`Actor.RootComponent` _array_element))))))
    (bind _returnvalue_3 (`KismetStringLibrary.Conv_DoubleToString` (.y (.scale (`SceneComponent.K2_GetComponentToWorld` (`Actor.RootComponent` _array_element))))))
    (bind _returnvalue_4 (`KismetStringLibrary.Conv_DoubleToString` (.z (.scale (`SceneComponent.K2_GetComponentToWorld` (`Actor.RootComponent` _array_element))))))
    (`KismetArrayLibrary.Array_Add` (`self.5_InternalDocument`) (`VictoryBPFunctionLibrary.AppendMultiple` (`VictoryBPFunctionLibrary.AppendMultiple` "InternalDocument") _seperatortype (`VictoryBPFunctionLibrary.AppendMultiple` _returnvalue) _seperatortype (`self.Creator`) _seperatortype (`VictoryBPFunctionLibrary.AppendMultiple` "An abstract Box in 3D-space representing a part of the building") _seperatortype (`VictoryBPFunctionLibrary.AppendMultiple` (`KismetTextLibrary.Conv_TextToString` (`/Game/Viewer/01_Core/01_Partonomie/BPO_BuildingPart.GetBuildingPartName` _boxcontainervariables_buildingpart))) _seperatortype (`VictoryBPFunctionLibrary.AppendMultiple` "Version 0.1") _seperatortype _seperatortype _seperatortype _seperatortype "3dBoxObject" _seperatortype (`self.GetDateTimeStringAppend`) _seperatortype (`self.Publisher`) _seperatortype "m" _seperatortype (`VictoryBPFunctionLibrary.AppendMultiple` (`KismetStringLibrary.Conv_DoubleToString` (/ (.x (.location (`SceneComponent.K2_GetComponentToWorld` (`Actor.RootComponent` _array_element)))) 100.0)) ", " (`KismetStringLibrary.Conv_DoubleToString` (/ (.y (.location (`SceneComponent.K2_GetComponentToWorld` (`Actor.RootComponent` _array_element)))) 100.0)) ", " (`KismetStringLibrary.Conv_DoubleToString` (/ (.z (.location (`SceneComponent.K2_GetComponentToWorld` (`Actor.RootComponent` _array_element)))) 100.0)) _seperatortype (`KismetStringLibrary.Conv_DoubleToString` (.roll (.rotation (`SceneComponent.K2_GetComponentToWorld` (`Actor.RootComponent` _array_element))))) ", " (`KismetStringLibrary.Conv_DoubleToString` (.pitch (.rotation (`SceneComponent.K2_GetComponentToWorld` (`Actor.RootComponent` _array_element))))) ", " (`KismetStringLibrary.Conv_DoubleToString` (.yaw (.rotation (`SceneComponent.K2_GetComponentToWorld` (`Actor.RootComponent` _array_element))))) _seperatortype _returnvalue_2 ", " _returnvalue_3 ", " _returnvalue_4 _seperatortype _returnvalue_2 ", " _returnvalue_3 ", " _returnvalue_4)))))

(fn `CreateBuildingPartStringArrays`
  (params (InputBuildingPartCollections :type "Array of /Game/Viewer/01_Core/01_Partonomie/BPO_BuildingPartCollection Object Reference"))
  (bind _seperatortype (`self.SeperatorType`))
  ;[1 1 1] Create BuildingPart StringArray
  (for _array_element InputBuildingPartCollections
    (bind (_buildingpartvariables_buildingpartid _buildingpartvariables_name) (break `/Game/Viewer/01_Core/Structs/S_BuildingPart` (`/Game/Viewer/01_Core/01_Partonomie/BPO_BuildingPart.BuildingPartVariables` _array_element)))
    (bind _returnvalue (`KismetGuidLibrary.Conv_GuidToString` _buildingpartvariables_buildingpartid))
    (`KismetArrayLibrary.Array_Add` (`self.InternalDocumentIDs`) _returnvalue)
    (`KismetArrayLibrary.Array_Add` (`self.5_InternalDocument`) (`VictoryBPFunctionLibrary.AppendMultiple` (`VictoryBPFunctionLibrary.AppendMultiple` "InternalDocument") _seperatortype (`VictoryBPFunctionLibrary.AppendMultiple` _returnvalue) _seperatortype (`self.Creator`) _seperatortype (`VictoryBPFunctionLibrary.AppendMultiple` "A part of the building hierarchy") _seperatortype (`VictoryBPFunctionLibrary.AppendMultiple` _buildingpartvariables_name) _seperatortype (`VictoryBPFunctionLibrary.AppendMultiple` "Version 0.1") _seperatortype (`VictoryBPFunctionLibrary.AppendMultiple` "") _seperatortype (`VictoryBPFunctionLibrary.AppendMultiple` "") _seperatortype (`VictoryBPFunctionLibrary.AppendMultiple` "") _seperatortype (`VictoryBPFunctionLibrary.AppendMultiple` "BuildingPartObject") _seperatortype (`VictoryBPFunctionLibrary.AppendMultiple` (`self.GetDateTimeStringAppend`)) _seperatortype (`self.Publisher`) (`VictoryBPFunctionLibrary.AppendMultiple` _seperatortype _seperatortype _seperatortype _seperatortype _seperatortype)))))

(fn `CreateLinkedFilesCollectionArrays`
  (params (InputLinkedFilesCollection :type "Array of /Game/Viewer/01_Core/00_LinkedDocuments/BP_LinkedFile Object Reference"))
  (bind _seperatortype (`self.SeperatorType`))
  ;[1 1 1] Create LinkedFiles StringArray
  (for _array_element InputLinkedFilesCollection
    (bind (_linkedfilevars_fileguid _linkedfilevars_filename _linkedfilevars_title _linkedfilevars_filepath _linkedfilevars_fileformat _linkedfilevars_documenttype _linkedfilevars_isplaced3d _linkedfilevars_3dactor _linkedfilevars_3dactorpointcloud _linkedfilevars_inserttransform _linkedfilevars_datetimeadded) (break `/Game/Viewer/01_Core/Structs/S_File` (`/Game/Viewer/01_Core/00_LinkedDocuments/BP_LinkedFile.LinkedFileVars` _array_element)))
    (`KismetArrayLibrary.Array_Add` (`self.InternalDocumentIDs`) (`KismetGuidLibrary.Conv_GuidToString` _linkedfilevars_fileguid))
    (bind (_year _month _day _hour _minute _second) (`KismetMathLibrary.BreakDateTime` _linkedfilevars_datetimeadded))
    (`KismetArrayLibrary.Array_Add` (`self.5_InternalDocument`) (`VictoryBPFunctionLibrary.AppendMultiple` (`VictoryBPFunctionLibrary.AppendMultiple` "InternalDocument") _seperatortype (`VictoryBPFunctionLibrary.AppendMultiple` (`KismetGuidLibrary.Conv_GuidToString` _linkedfilevars_fileguid)) _seperatortype (`self.Creator`) _seperatortype (`VictoryBPFunctionLibrary.AppendMultiple` "A file linked to a part of a building") (`VictoryBPFunctionLibrary.AppendMultiple` "" _seperatortype) (`VictoryBPFunctionLibrary.AppendMultiple` _linkedfilevars_title) _seperatortype (`VictoryBPFunctionLibrary.AppendMultiple` "Version 0.1") _seperatortype _seperatortype _seperatortype _linkedfilevars_filename _seperatortype (`VictoryBPFunctionLibrary.AppendMultiple` (`.RightS` (`KismetStringLibrary.Split` _linkedfilevars_filename "." "IgnoreCase" "FromEnd"))) _seperatortype (`VictoryBPFunctionLibrary.AppendMultiple` (`VictoryBPFunctionLibrary.AppendMultiple` (`KismetStringLibrary.Conv_IntToString` _year) "-" (`KismetStringLibrary.Conv_IntToString` _month) "-" (`KismetStringLibrary.Conv_IntToString` _day) "T" (`KismetStringLibrary.Conv_IntToString` _hour) ":" (`KismetStringLibrary.Conv_IntToString` _minute) ":" (`KismetStringLibrary.Conv_IntToString` _second))) _seperatortype (`self.Publisher`) _seperatortype _seperatortype _seperatortype))))

(fn `GetDateTimeStringAppend`
  (returns (ReturnValue :type String))
  (bind (_year _month _day _hour _minute _second) (`KismetMathLibrary.BreakDateTime` (`KismetMathLibrary.Now`)))
  (return (`VictoryBPFunctionLibrary.AppendMultiple` (`KismetStringLibrary.Conv_IntToString` _year) "-" (`KismetStringLibrary.Conv_IntToString` _month) "-" (`KismetStringLibrary.Conv_IntToString` _day) "T" (`KismetStringLibrary.Conv_IntToString` _hour) ":" (`KismetStringLibrary.Conv_IntToString` _minute) ":" (`KismetStringLibrary.Conv_IntToString` _second))))

(fn `UserConstructionScript`)